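; Default player controller that provides debug hotkeys for a preview actor with avatar head and body bone info.
; H toggles the visibility of the preview actor's widget.
; NumPad 0 dumps new bone categories and the numpad decimal key dumps new bone keys, both through the head and body AvatarBoneInfo objects.
; BeginPlay, Tick and the construction script are empty, and the preview actor reference is not assigned here.
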(event `Key|H`
  (params (Key :type "Key Structure" :default "AnyKey"))
  (bind _widget (`/Game/Cosmetic/PreviewActor.Widget` (`self.PreviewActor`)))
  (:`Pressed`
    (if (`Widget.IsVisible` _widget)
      (`Widget.SetVisibility` _widget "Hidden")
      (else
        (`Widget.SetVisibility` _widget "Visible")))))

(event `Key|NumPadZero`
  (params (Key :type "Key Structure" :default "AnyKey"))
  (bind _headavatarboneinfo (`/Game/Cosmetic/PreviewActor.HeadAvatarBoneInfo` (`self.PreviewActor`)))
  (:`Pressed`
    (`AvatarBoneInfo.DumpNewBoneCategory` _headavatarboneinfo)
    (`AvatarBoneInfo.DumpNewBoneCategory` _headavatarboneinfo)
    (`AvatarBoneInfo.DumpNewBoneCategory` (`/Game/Cosmetic/PreviewActor.BodyAvatarBoneInfo` (`self.PreviewActor`)))))

(event `Key|Decimal`
  (params (Key :type "Key Structure" :default "AnyKey"))
  (bind _previewactor (`self.PreviewActor`))
  (:`Pressed`
    (`AvatarBoneInfo.DumpNewBoneKeys` (`/Game/Cosmetic/PreviewActor.HeadAvatarBoneInfo` _previewactor))
    (`AvatarBoneInfo.DumpNewBoneKeys` (`/Game/Cosmetic/PreviewActor.BodyAvatarBoneInfo` _previewactor))))

(fn `UserConstructionScript`)